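; BP_Cell_Scoring is a board cell Blueprint that awards 10 points to a player when its action runs.
; Its Action override calls the parent, then rewrites that player's entry in the game instance's PlayerList with the increased score, using PlayerId as the array index.
; The event graph is disabled, and the construction script holds only unconnected leftover scoring and pawn-move nodes.
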(event EventBeginPlay
  (|CallParentFunction) ; This node is disabled and will not be called.\nDrag off pins to build functionality.
)

(event Collision|EventActorBeginOverlap
  (params (OtherActor :type Actor%20Object%20Reference)))

(event EventTick
  (params (DeltaSeconds :type Float%20%28single-precision%29)))

(fn ConstructionScript)

(fn Action
  (params (PlayerId :type Integer))
  (bind _as_bp_game_instance (Variables|Default|GetAs%20BP%20Game%20Instance))
  (bind _playerlist (Variables|/Game/Blueprints/BP_GameInstance.BP_GameInstance_C|GetPlayerList _as_bp_game_instance))
  (bind _output (Utilities|Array|Get(acopy) _playerlist PlayerId))
  (bind (_playerid _score _cellnumber) (Utilities|Struct|BreakS_PlayerData _output))
  (|CallParentFunction PlayerId)
  (Utilities|Array|SetArrayElem _playerlist PlayerId (Utilities|Struct|MakeS_PlayerData _playerid (+ _score 10) _cellnumber)))